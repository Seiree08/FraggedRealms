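; BP_Paddle is the player-controlled paddle for the BrickBreaker game.
; On BeginPlay it registers the BrickBreaker Enhanced Input mapping context with its player controller, then creates the WB_BrickBreaker HUD and adds it to the viewport.
; The move input action shifts the Paddle component along its local Z axis, scaled by PaddleSpeed but not by delta time.
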(event Input|EnhancedActionEvents|EnhancedInputActionIA_PaddleMove
  (params (ActionValue :type Float%20%28double-precision%29) (ElapsedSeconds :type Float%20%28double-precision%29) (TriggeredSeconds :type Float%20%28double-precision%29) (InputAction :type Input%20Action%20Object%20Reference :default "/Game/BrickBreaker/Input/IA_PaddleMove.IA_PaddleMove"))
  (Transformation|AddLocalOffset (Variables|Default|GetPaddle) (Math|Vector|MakeVector 0.0 0.0 (* ActionValue (Variables|Default|GetPaddleSpeed))) false false))

(event EventBeginPlay
  (bind _asplayer_controller (Utilities|Casting|CastToPlayerController (Pawn|GetController)))
  (Utilities|IsValid (PlayerController|LocalPlayerSubsystems|GetEnhancedInputLocalPlayerSubsystem _asplayer_controller)
    (:Is%20Valid
      (Input|AddMappingContext (PlayerController|LocalPlayerSubsystems|GetEnhancedInputLocalPlayerSubsystem _asplayer_controller) "/Game/BrickBreaker/Input/IMC_BrickBreaker.IMC_BrickBreaker" 0 "(bIgnoreAllPressedKeysUntilRelease=True,bForceImmediately=False,bNotifyUserSettings=False)")
      (bind _returnvalue (UserInterface|CreateWidget "/Game/BrickBreaker/Blueprints/WB_BrickBreaker.WB_BrickBreaker_C"))
      (bind _output_get (Variables|Default|SetBrickHUD _returnvalue))
      (UserInterface|Viewport|AddtoViewport _output_get 0))))

(event Collision|EventActorBeginOverlap
  (params (OtherActor :type Actor%20Object%20Reference)))

(event EventTick
  (params (DeltaSeconds :type Float%20%28single-precision%29)))

(fn ConstructionScript)